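; Idle ability for the turn-based tile toolkit that lets a player click grid units to select them.
; On a released click on a valid tile, the server-side interact event checks that the first actor in the initiative order shares the ability's owner.
; It then selects the clicked unit if it is player-controlled, has that owner, will act this turn and precedes any next faction in the initiative order.
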(event `self.ServerInteract`
  (params (bValidTile :type Boolean) (Index :type Integer) (Location :type "Vector Structure") (Key :type "Key Structure") (bReleased :type Boolean) (ClickType :type "/Game/AdvancedTurnBasedTileToolkit/Core/Grid/EClickType Enum" :default "NewEnumerator0") (CallingPc :type "/Game/AdvancedTurnBasedTileToolkit/Core/BP_PlayerController_ATBTT Object Reference"))
  (bind (_value _returnvalue) (`BlueprintMapLibrary.Map_Find` (`/Game/AdvancedTurnBasedTileToolkit/Core/Grid/BP_GridManager.GridUnits` (`self.GridManagerRef`)) (`self.ClickedIndex`)))
  (bind _value_2 (`BlueprintMapLibrary.Map_Find` (`/Game/AdvancedTurnBasedTileToolkit/Core/Grid/BP_GridManager.GridUnits` (`self.GridManagerRef`)) (`self.ClickedIndex`)))
  (if bValidTile
    (if bReleased
      (switch `/Game/AdvancedTurnBasedTileToolkit/Core/Grid/EClickType` "NewEnumerator0"
        (:`NewEnumerator0`
          (bind _turnmanager (message `/Game/AdvancedTurnBasedTileToolkit/Core/BPI_Singletons.GetTurnManager` (`GameplayStatics.GetGameState`)))
          (if (== (`self.GetOwner` (`|GetArrayItem` (`/Game/AdvancedTurnBasedTileToolkit/Core/BP_TurnManager.InitiativeOrderActors` _turnmanager))) (`self.GetOwner`))
            (if _returnvalue
              (if (and (not (`/Game/AdvancedTurnBasedTileToolkit/Core/Units/BP_Unit.bAIControlled` _value)) (== (`self.GetOwner` _value) (`self.GetOwner`)))
                (bind _turnmanager_2 (message `/Game/AdvancedTurnBasedTileToolkit/Core/BPI_Singletons.GetTurnManager` (`GameplayStatics.GetGameState`)))
                (bind _bwillact (`/Game/AdvancedTurnBasedTileToolkit/Core/BP_TurnManager.CheckIfActorWillActThisTurn` _turnmanager_2 _value_2))
                (if _bwillact
                  (bind (_bsuccess _index) (`/Game/AdvancedTurnBasedTileToolkit/Core/BP_TurnManager.FindIndexOfNextFaction` _turnmanager_2))
                  (if (or (not _bsuccess) (> _index (`KismetArrayLibrary.Array_Find` (`/Game/AdvancedTurnBasedTileToolkit/Core/BP_TurnManager.InitiativeOrderActors` _turnmanager_2) _value_2)))
                    (message `/Game/AdvancedTurnBasedTileToolkit/Core/BPI_Initiative.SelectActor` (`BlueprintMapLibrary.Map_Find` (`/Game/AdvancedTurnBasedTileToolkit/Core/Grid/BP_GridManager.GridUnits` (`self.GridManagerRef`)) (`self.ClickedIndex`)))))))))))))

(fn `UserConstructionScript`
  (`parent.UserConstructionScript`))