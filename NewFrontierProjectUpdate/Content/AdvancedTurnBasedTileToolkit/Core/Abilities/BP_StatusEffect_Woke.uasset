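; BP_StatusEffect_Woke is a status effect for the turn-based tile toolkit that flags its owning unit as woken.
; On activation it pans the player pawn's view to the unit, reveals the effect indicator and plays a discovery sound.
; Timed delays pace this presentation before it tells the game state to end the action.
; The effect disables itself when its turn-start event runs.
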(event `self.AnimateActivation`
  (bind _returnvalue (`self.K2_GetActorLocation` (`self.OwningUnit`)))
  (message `/Game/AdvancedTurnBasedTileToolkit/Core/BPI_CameraControls.PanToLocation` (`GameplayStatics.GetPlayerPawn` 0) _returnvalue)
  (`KismetSystemLibrary.Delay` 0.6)
  (`SceneComponent.SetVisibility` (`self.EffectIndicator`) true false)
  (`GameplayStatics.PlaySoundAtLocation` "/Game/AdvancedTurnBasedTileToolkit/Core/Abilities/A_Discover.A_Discover" _returnvalue (struct) 1.0 1.0 0.0 null null null)
  (`KismetSystemLibrary.Delay` 1.0)
  (message `/Game/AdvancedTurnBasedTileToolkit/Core/BPI_Action.EndAction` (`GameplayStatics.GetGameState`)))

(event `self.RunOnTurnStart`
  (`self.Disable`))

(fn `UserConstructionScript`
  (`parent.UserConstructionScript`))