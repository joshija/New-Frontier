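; BP_GridActor is an actor that aligns itself to the tile grid of the level's BP_GridManager.
; With AutoGridPlacement on, its construction script derives GridIndex from the closest traced tile.
; If custom-grid snapping applies, it attaches to or detaches from the manager and snaps only the GridAnchor component, carrying the mesh, to that tile plus AnchorOffset.
; PlaceActorAtAnchor moves the actor itself to the anchor, then re-snaps the anchor.
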(fn `PlaceActorAtAnchor`
  (`self.K2_SetActorLocation` (`SceneComponent.K2_GetComponentLocation` (`self.GridAnchor`)))
  (bind _snaplocation (`/Game/AdvancedTurnBasedTileToolkit/Core/Grid/BP_GridManager.FindClosestTileToSnapToTrace` (`self.GridManagerRef`) (`self.K2_GetActorLocation`)))
  (`SceneComponent.K2_SetWorldLocation` (`self.GridAnchor`) (+ _snaplocation (`self.AnchorOffset`)) false false)
  (return))

(fn `UserConstructionScript`
  (bind _outactors (`GameplayStatics.GetAllActorsOfClass` "/Game/AdvancedTurnBasedTileToolkit/Core/Grid/BP_GridManager.BP_GridManager_C")) ; Get a referance to the Grid Manager
  (if (> (`KismetArrayLibrary.Array_Length` _outactors) 0)
    (set `self.GridManagerRef` (`|GetArrayItem` _outactors))
    (if (`self.bAutoGridPlacement`)
      (bind _snaplocation (`/Game/AdvancedTurnBasedTileToolkit/Core/Grid/BP_GridManager.FindClosestTileToSnapToTrace` (`self.GridManagerRef`) (`self.K2_GetActorLocation`)))
      (set `self.GridIndex` (`/Game/AdvancedTurnBasedTileToolkit/Core/Grid/BP_GridManager.ConvertLocationToIndex3D` (`self.GridManagerRef`) (- _snaplocation (`self.AnchorOffset`))))
      (if (`/Game/AdvancedTurnBasedTileToolkit/Core/Grid/BP_GridManager.bSnapToCustomGrid` (`self.GridManagerRef`))
        (if (not (`self.bIgnoreSnapToCustomGrid`))
          (if (`self.bAttachOnConstruction`)
            (`self.K2_AttachToActor` (`self.GridManagerRef`) "None" "KeepWorld" "SnapToTarget" "SnapToTarget")
            (else
              (`self.K2_DetachFromActor` self "KeepWorld" "KeepWorld" "KeepWorld")))
          (bind _snaplocation_2 (`/Game/AdvancedTurnBasedTileToolkit/Core/Grid/BP_GridManager.FindClosestTileToSnapToTrace` (`self.GridManagerRef`) (`self.K2_GetActorLocation`)))
          (`SceneComponent.K2_SetWorldLocation` (`self.GridAnchor`) (+ _snaplocation_2 (`self.AnchorOffset`)) false false) ; Set the location of the anchor which the mesh is tied to. Even though the actor is at the same position, the mesh will snap to the grid.
        )))))