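; 2D snail unit for the turn-based tile toolkit that is meant to lose its shell visually once wounded.
; TakeDamage checks the health ratio before calling the parent, so the first hit received at or below the threshold queues a one-time lose-shell action.
; AnimateAction handles the shell-loss action by swapping the unit sprite to the snail sprite and passes other actions to the parent.
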(event `self.TakeDamage`
  (params (Damage :type "Float (single-precision)") (bAutoAnimate :type Boolean))
  (if (<= (/ (`self.CurrentHealth`) (`self.MaxHealth`)) 0.7)
    (`|ExecutionSequence`
      (:`then_0`
        (`/Engine/EditorBlueprintResources/StandardMacros.DoOnce` false
          (:`Completed`
            (`/Game/AdvancedTurnBasedTileToolkit/Core/BPML_ATBTT.QueueAction` false self "LoseShell" true))))
      (:`then_1`
        (`parent.TakeDamage` Damage bAutoAnimate :!label _label)))
    (else
      (goto _label))))

(event `/Game/AdvancedTurnBasedTileToolkit/Core/BPI_Action.AnimateAction`
  (params (Action :type "/Game/AdvancedTurnBasedTileToolkit/Core/FAction Structure"))
  (switch `name` (`.ActionName_37_58E425AA41088A6D07425C9F0FBA2C3F` (break `/Game/AdvancedTurnBasedTileToolkit/Core/FAction` Action))
    (:`Default`
      (`parent.AnimateAction` Action))
    (:`LoseShell`
      (`PaperSpriteComponent.SetSprite` (`self.UnitSprite`) "/Game/AdvancedTurnBasedTileToolkit/Maps/2D/Units/SPR_Snail.SPR_Snail"))))

(fn `UserConstructionScript`
  (`parent.UserConstructionScript`))