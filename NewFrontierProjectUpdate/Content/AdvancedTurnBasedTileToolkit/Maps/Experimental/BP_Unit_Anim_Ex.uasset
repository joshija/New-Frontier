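; Experimental animated unit for the tile toolkit that adds jump and teleport traversal to grid movement.
; SimulateMove splits paths at GridManager special edges, queuing MoveSegment, Jump (also used for climbs) and Teleport actions.
; AnimateAction plays them: speed-eased spline movement with optional ground tracing, a timeline jump arc, or a delayed teleport with particles.
; Moves and jumps feed speed to the AnimBP; each action notifies the GameState when done.
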(event `self.MoveToIndex`
  (params (IndexPathEnd :type Integer) (PathsMap :type "Map of Integer to /Game/AdvancedTurnBasedTileToolkit/Core/Grid/FPathfindingNew Structure (by ref)"))
  (bind _pathindexes (`/Game/AdvancedTurnBasedTileToolkit/Core/Grid/BP_GridManager.FindSplinePathToGridIndex` (`self.GridManagerRef`) PathsMap IndexPathEnd (`self.AnchorOffset`) null "Curve"))
  (`self.SimulateMove` _pathindexes))

(event `/Game/AdvancedTurnBasedTileToolkit/Core/BPI_Action.AnimateAction`
  (params (Action :type "/Game/AdvancedTurnBasedTileToolkit/Core/FAction Structure"))
  ;[1 0.2858 0] AnimateAction
  (switch `name` (`.ActionName_37_58E425AA41088A6D07425C9F0FBA2C3F` (break `/Game/AdvancedTurnBasedTileToolkit/Core/FAction` Action))
    (:`Default`
      (`parent.AnimateAction` Action))
    (:`MoveSegment`
      (`self.MoveSegment` Action))
    (:`Jump`
      (`self.Jump` Action))
    (:`Teleport`
      (`self.Teleport` Action))))

(event `MoveSegment`
  (params (Action :type "/Game/AdvancedTurnBasedTileToolkit/Core/FAction Structure"))
  (bind (_executingobject _actionname _binstantdeactivate _atcustomindex _bwithprevious _activationdelay _booleans _integers _floats _strings _vectors) (break `/Game/AdvancedTurnBasedTileToolkit/Core/FAction` Action))
  (bind _returnvalue (`self.K2_GetActorLocation`))
  (bind _currentsplinedistance (`self.CurrentSplineDistance`))
  (bind _spline (`/Game/AdvancedTurnBasedTileToolkit/Core/Units/BP_PathSpline.Spline` (`self.PathSplineRef`)))
  (bind _spline_2 (`/Game/AdvancedTurnBasedTileToolkit/Core/Units/BP_PathSpline.Spline` (`self.PathSplineRef`)))
  (bind (_returnvalue_x _returnvalue_y _returnvalue_z) (`KismetMathLibrary.BreakVector` (`SplineComponent.GetLocationAtDistanceAlongSpline` (`/Game/AdvancedTurnBasedTileToolkit/Core/Units/BP_PathSpline.Spline` (`self.PathSplineRef`)) (`self.CurrentSplineDistance`) "World")))
  (bind _returnvalue_2 (`SplineComponent.GetDistanceAlongSplineAtSplinePoint` _spline_2 0))
  (bind _returnvalue_3 (* (`SceneComponent.GetUpVector` (`self.GridAnchor`)) (/ (.z (`.BoxExtent` (`KismetSystemLibrary.GetComponentBounds` (`self.Mesh`)))) 2.0)))
  (bind _returnvalue_4 (`SplineComponent.GetDistanceAlongSplineAtSplinePoint` _spline_2 (- (`SplineComponent.GetNumberOfSplinePoints` _spline) 1)))
  ;[1 0.2858 0] AnimateAction
  (`SplineComponent.SetSplinePoints` _spline _vectors "World" true)
  (set `self.CurrentSplineDistance` _returnvalue_2)
  (`/Game/AdvancedTurnBasedTileToolkit/Core/BPML_ATBTT.WhileLoop_Delayed` (< (`self.CurrentSplineDistance`) _returnvalue_4)
    (:`Loop Body`
      (set `self.CurrentSpeed` (`KismetMathLibrary.FMin` (`KismetMathLibrary.FMin` (`self.MaxSpeed`) _returnvalue_4) (`KismetMathLibrary.SelectFloat` (`KismetMathLibrary.FMax` (* (- _returnvalue_4 _currentsplinedistance) 6.0) 200.0) (`self.MaxSpeed`) (`|GetArrayItem` _booleans)) (`KismetMathLibrary.FMax` (* (- _currentsplinedistance _returnvalue_2) 6.0) 200.0)))
      (bind _output_get (set `self.CurrentSplineDistance` (+ (* (`GameplayStatics.GetWorldDeltaSeconds`) (`self.CurrentSpeed`)) (`self.CurrentSplineDistance`))))
      (`self.K2_SetActorRelativeRotation` (`KismetMathLibrary.MakeRotator` 0.0 0.0 (.yaw (`SplineComponent.GetRotationAtDistanceAlongSpline` (`/Game/AdvancedTurnBasedTileToolkit/Core/Units/BP_PathSpline.Spline` (`self.PathSplineRef`)) _output_get "World"))))
      (if (`self.bTraceForGround`)
        (bind (_outhit _returnvalue_5) (`KismetSystemLibrary.LineTraceSingle` (+ _returnvalue _returnvalue_3) (- _returnvalue _returnvalue_3) "TraceTypeQuery3")))
      (`self.K2_SetActorLocation` (`KismetMathLibrary.MakeVector` _returnvalue_x _returnvalue_y (`KismetMathLibrary.SelectFloat` (.z (`.Location` (`GameplayStatics.BreakHitResult` _outhit))) _returnvalue_z (and (`self.bTraceForGround`) _returnvalue_5))))
      (message `/Game/AdvancedTurnBasedTileToolkit/Core/BPI_AnimateUnit.AnimateMovement` (`self.AbpRef`) (`self.CurrentSpeed`)))
    (:`Completed`
      (message `/Game/AdvancedTurnBasedTileToolkit/Core/BPI_AnimateUnit.AnimateMovement` (`self.AbpRef`) 0.0)
      (message `/Game/AdvancedTurnBasedTileToolkit/Core/BPI_Action.EndAction` (`GameplayStatics.GetGameState`)))))

(event `Jump`
  (params (Action :type "/Game/AdvancedTurnBasedTileToolkit/Core/FAction Structure"))
  (bind (_executingobject _actionname _binstantdeactivate _atcustomindex _bwithprevious _activationdelay _booleans _integers _floats _strings _vectors) (break `/Game/AdvancedTurnBasedTileToolkit/Core/FAction` Action))
  (bind _output (`|GetArrayItem` _vectors))
  (bind _output_2 (`|GetArrayItem` _vectors 1))
  ;[1 0.2858 0] AnimateAction
  (`/Game/AdvancedTurnBasedTileToolkit/Core/BPML_ATBTT.SimpleQueue` true self "JumpAnim" true)
  (bind (_direction _time _height) (`Timeline|TL_Jump` :!via `PlayFromStart`)
    (:`Update`
      (`self.K2_SetActorRelativeRotation` (`KismetMathLibrary.MakeRotator` 0.0 0.0 (.yaw (`KismetMathLibrary.FindLookAtRotation` _output _output_2))))
      (bind (_returnvalue_x _returnvalue_y _returnvalue_z) (`KismetMathLibrary.BreakVector` (`KismetMathLibrary.VLerp` _output _output_2 _time)))
      (`self.K2_SetActorLocation` (`KismetMathLibrary.MakeVector` _returnvalue_x _returnvalue_y (+ (* _height 200.0) _returnvalue_z)))
      (message `/Game/AdvancedTurnBasedTileToolkit/Core/BPI_AnimateUnit.AnimateMovement` (`self.AbpRef`) 400.0))
    (:`Finished`
      (message `/Game/AdvancedTurnBasedTileToolkit/Core/BPI_AnimateUnit.AnimateMovement` (`self.AbpRef`) 0.0)
      (message `/Game/AdvancedTurnBasedTileToolkit/Core/BPI_Action.EndAction` (`GameplayStatics.GetGameState`)))))

(event `Teleport`
  (params (Action :type "/Game/AdvancedTurnBasedTileToolkit/Core/FAction Structure"))
  ;[1 0.2858 0] AnimateAction
  (`KismetSystemLibrary.Delay` 0.5)
  (`GameplayStatics.SpawnEmitterAtLocation` "/Game/AdvancedTurnBasedTileToolkit/Maps/Advanced/Abilities/PS_Explosion.PS_Explosion" (`self.K2_GetActorLocation`) (struct) (4.0 4.0 4.0))
  (`self.SetActorHiddenInGame` true)
  (`KismetSystemLibrary.Delay` 0.5)
  (`self.K2_SetActorLocation` (`|GetArrayItem` (`.Vectors_46_AF930FE8427632CA6CD1B994AE42A291` (break `/Game/AdvancedTurnBasedTileToolkit/Core/FAction` Action))))
  (`KismetSystemLibrary.Delay` 0.5)
  (`GameplayStatics.SpawnEmitterAtLocation` "/Game/AdvancedTurnBasedTileToolkit/Maps/Advanced/Abilities/PS_Explosion.PS_Explosion" (`self.K2_GetActorLocation`) (struct) (4.0 4.0 4.0))
  (`self.SetActorHiddenInGame` false)
  (`KismetSystemLibrary.Delay` 0.5)
  (message `/Game/AdvancedTurnBasedTileToolkit/Core/BPI_Action.EndAction` (`GameplayStatics.GetGameState`)))

(fn `QueueMoveSegment`
  (params (bHaltOnEnd :type Boolean) (PathLocations :type "Array of Vector Structure (by ref)"))
  (if (> (`KismetArrayLibrary.Array_Length` PathLocations) 1)
    (`/Game/AdvancedTurnBasedTileToolkit/Core/BPML_ATBTT.QueueAction` :`Executing Object` self :`Action Name` "MoveSegment" :`Booleans` (`|MakeArray` bHaltOnEnd) :`Vectors` (`local.PathLocations`))
    (return)
    (else
      (return))))

(fn `SimulateMove`
  (params (PathIndexes :type "Array of Integer (by ref)"))
  (returns (NewActionsCount :type Integer) (bInterrupted :type Boolean))
  (locals (CurrentIndex :type Integer) (NextIndex :type Integer) (LocalPathLocations :type "Array of Vector Structure"))
  (bind (_value _returnvalue) (`BlueprintMapLibrary.Map_Find` (`/Game/AdvancedTurnBasedTileToolkit/Core/Grid/BP_GridManager.SpecialEdges` (`self.GridManagerRef`)) (`local.CurrentIndex`)))
  (bind (_value_2 _returnvalue_2) (`BlueprintMapLibrary.Map_Find` (break `/Game/AdvancedTurnBasedTileToolkit/Core/Grid/FSpecialEdges` _value) (`local.NextIndex`)))
  (bind (_newactionscount _binterrupted) (`parent.SimulateMove` PathIndexes))
  (`|ExecutionSequence`
    (:`then_0`
      (`KismetArrayLibrary.Array_Add` (`local.LocalPathLocations`) (`BlueprintMapLibrary.Map_Find` (`/Game/AdvancedTurnBasedTileToolkit/Core/Grid/BP_GridManager.GridLocations` (`self.GridManagerRef`)) (`|GetArrayItem` PathIndexes)))
      (for (_array_element _array_index) PathIndexes
        (set `local.CurrentIndex` _array_element)
        (if (< _array_index (`KismetArrayLibrary.Array_LastIndex` (`local.PathIndexes`)))
          (set `local.NextIndex` (`|GetArrayItem` (`local.PathIndexes`) (+ _array_index 1)))
          (`|ExecutionSequence`
            (:`then_0`
              (if _returnvalue
                (if _returnvalue_2
                  (bind ___ (`/Game/AdvancedTurnBasedTileToolkit/Core/BPML_ATBTT.MakeLocalVariable` _value_2))
                  (switch `/Game/AdvancedTurnBasedTileToolkit/Core/Grid/ESpecialEdge` ___
                    (:`NewEnumerator1`
                      _)
                    (:`NewEnumerator2`
                      _)
                    (:`NewEnumerator3`
                      _)
                    (:`NewEnumerator4`
                      _))
                  (`|ExecutionSequence`
                    (:`then_0`
                      (`self.QueueMoveSegment` (select `/Game/AdvancedTurnBasedTileToolkit/Core/Grid/ESpecialEdge` ___ :`NewEnumerator0` true :`NewEnumerator4` true) (`local.LocalPathLocations`)))
                    (:`then_1`
                      (`KismetArrayLibrary.Array_Clear` (`local.LocalPathLocations`))
                      (switch `/Game/AdvancedTurnBasedTileToolkit/Core/Grid/ESpecialEdge` ___
                        (:`NewEnumerator1`
                          (`/Game/AdvancedTurnBasedTileToolkit/Core/BPML_ATBTT.QueueAction` :`Executing Object` self :`Action Name` "Jump" :`Vectors` (`|MakeArray` (`BlueprintMapLibrary.Map_Find` (`/Game/AdvancedTurnBasedTileToolkit/Core/Grid/BP_GridManager.GridLocations` (`self.GridManagerRef`)) (`local.CurrentIndex`)) (`BlueprintMapLibrary.Map_Find` (`/Game/AdvancedTurnBasedTileToolkit/Core/Grid/BP_GridManager.GridLocations` (`self.GridManagerRef`)) (`local.NextIndex`))) :!label _label))
                        (:`NewEnumerator2`
                          (goto _label))
                        (:`NewEnumerator3`
                          (goto _label))
                        (:`NewEnumerator4`
                          (`/Game/AdvancedTurnBasedTileToolkit/Core/BPML_ATBTT.QueueAction` :`Executing Object` self :`Action Name` "Teleport" :`Vectors` (`|MakeArray` (`BlueprintMapLibrary.Map_Find` (`/Game/AdvancedTurnBasedTileToolkit/Core/Grid/BP_GridManager.GridLocations` (`self.GridManagerRef`)) (`local.NextIndex`)))))))))))
            (:`then_1`
              (`KismetArrayLibrary.Array_Add` (`local.LocalPathLocations`) (`BlueprintMapLibrary.Map_Find` (`/Game/AdvancedTurnBasedTileToolkit/Core/Grid/BP_GridManager.GridLocations` (`self.GridManagerRef`)) (`local.NextIndex`)))))
          (else
            (`self.QueueMoveSegment` true (`local.LocalPathLocations`))))))
    (:`then_1`
      (return _newactionscount _binterrupted))))

(fn `UserConstructionScript`
  (`parent.UserConstructionScript`))