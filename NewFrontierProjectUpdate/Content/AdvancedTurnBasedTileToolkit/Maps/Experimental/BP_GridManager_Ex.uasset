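; Experimental grid manager variant that adds jump-down pathfinding edges, linking elevated tiles to lower ground.
; After the parent builds the grid arrays, it checks every tile in the edge map that sits high enough above the minimum grid height.
; Downward line traces at offsets around each tile find drops exceeding the impassable height cutoff.
; Each landing tile gets a cost-1 edge from the upper tile, tagged as a special edge.
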(event `self.SetupGridArrays`
  (`parent.SetupGridArrays`)
  (bind _keys (`BlueprintMapLibrary.Map_Keys` (`self.GridEdgesMap`)))
  (for _array_element _keys
    (`self.AddJumpDownEdges` _array_element (`BlueprintMapLibrary.Map_Find` (`self.GridLocations`) _array_element))))

(fn `AddJumpDownEdges`
  (params (GridIndex :type Integer) (GridLocation :type "Vector Structure"))
  (bind (_gridlocation_x _gridlocation_y _gridlocation_z) (`KismetMathLibrary.BreakVector` (`local.GridLocation`)))
  (if (> (.z GridLocation) (+ (`self.MinGridHeight`) (`self.HeightImpassableCutoff`)))
    (for _array_element (`self.TraceLocations`)
      (bind _returnvalue (+ _array_element (`local.GridLocation`)))
      (bind (_outhit _returnvalue_2) (`KismetSystemLibrary.LineTraceSingle` :`Start` _returnvalue :`End` (- _returnvalue (0.0 0.0 5000.0)) :`TraceChannel` "TraceTypeQuery3" :`bIgnoreSelf` false))
      (if _returnvalue_2
        (if (> (- _gridlocation_z (.z (`.Location` (`GameplayStatics.BreakHitResult` _outhit)))) (`self.HeightImpassableCutoff`))
          (bind ___ (`/Game/AdvancedTurnBasedTileToolkit/Core/BPML_ATBTT.MakeLocalVariable` (`self.ConvertLocationToIndex3D` (`.Location` (`GameplayStatics.BreakHitResult` _outhit)))))
          (`self.AddEdge` (`local.GridIndex`) ___)
          (`self.AddSpecialEdge` (`local.GridIndex`) ___ "NewEnumerator3"))))
    (return)
    (else
      (return))))

(fn `UserConstructionScript`
  (`parent.UserConstructionScript`))